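; KBMPawn is a pawn controlled by keyboard and mouse for movement and looking around.
; MoveForward and MoveRight axis inputs add movement along the actor's forward and right vectors.
; MouseX drives controller yaw, while MouseY drives pitch with its sign inverted by subtracting twice the axis value.
; The construction script is empty.
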(event Input|AxisEvents|InputAxisMoveForward
  (params (AxisValue :type Float%20%28single-precision%29))
  ;[1 1 1] KBM based
  (Pawn|Input|AddMovementInput (Transformation|GetActorForwardVector) AxisValue false))

(event Input|AxisEvents|InputAxisMoveRight
  (params (AxisValue :type Float%20%28single-precision%29))
  ;[1 1 1] KBM based
  (Pawn|Input|AddMovementInput (Transformation|GetActorRightVector) AxisValue false))

(event Input|MouseEvents|MouseX
  (params (AxisValue :type Float%20%28single-precision%29))
  ;[1 1 1] KBM based
  (Pawn|Input|AddControllerYawInput AxisValue))

(event Input|MouseEvents|MouseY
  (params (AxisValue :type Float%20%28single-precision%29))
  ;[1 1 1] KBM based
  (Pawn|Input|AddControllerPitchInput (- AxisValue (* 2 AxisValue))))

(fn ConstructionScript)