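; Door Blueprint that swings open when a BP_VRVisitor enters its Box trigger and closes when the visitor leaves.
; The OpenDoor timeline plays or reverses on overlap, scaling its curve by Angle to rotate the Door in relative yaw or pitch, chosen by ZTrueYFalse.
; On timeline finish, the direction decides Door collision: disabled once fully open, restored to query and physics once closed.
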(event OnComponentBeginOverlap(Box)
  (params (OverlappedComponent :type Primitive%20Component%20Object%20Reference) (OtherActor :type Actor%20Object%20Reference) (OtherComp :type Primitive%20Component%20Object%20Reference) (OtherBodyIndex :type Integer) (bFromSweep :type Boolean) (SweepResult :type Hit%20Result%20Structure%20%28by%20ref%29))
  (Utilities|Casting|CastToBP_VRVisitor OtherActor)
  (bind (_direction _fvalue) (Timeline|Open%20Door Play)
    (:Update
      (if (Variables|Default|GetZTrueYFalse)
        (Transformation|SetRelativeRotation (Variables|Default|GetDoor) (Math|Rotator|MakeRotator 0.0 0.0 (* _fvalue (Variables|Default|GetAngle))) false false)
        (else
          (Transformation|SetRelativeRotation (Variables|Default|GetDoor) (Math|Rotator|MakeRotator 0.0 (* _fvalue (Variables|Default|GetAngle)) 0.0) false false))))
    (:Finished
      (if (== (Math|Conversions|ToInteger(Byte) _direction) 0)
        (Collision|SetCollisionEnabled (Variables|Default|GetDoor) "NoCollision")
        (else
          (Collision|SetCollisionEnabled (Variables|Default|GetDoor) "QueryAndPhysics"))))))

(event OnComponentEndOverlap(Box)
  (params (OverlappedComponent :type Primitive%20Component%20Object%20Reference) (OtherActor :type Actor%20Object%20Reference) (OtherComp :type Primitive%20Component%20Object%20Reference) (OtherBodyIndex :type Integer))
  (Utilities|Casting|CastToBP_VRVisitor OtherActor)
  (bind (_direction _fvalue) (Timeline|Open%20Door Reverse)
    (:Update
      (if (Variables|Default|GetZTrueYFalse)
        (Transformation|SetRelativeRotation (Variables|Default|GetDoor) (Math|Rotator|MakeRotator 0.0 0.0 (* _fvalue (Variables|Default|GetAngle))) false false)
        (else
          (Transformation|SetRelativeRotation (Variables|Default|GetDoor) (Math|Rotator|MakeRotator 0.0 (* _fvalue (Variables|Default|GetAngle)) 0.0) false false))))
    (:Finished
      (if (== (Math|Conversions|ToInteger(Byte) _direction) 0)
        (Collision|SetCollisionEnabled (Variables|Default|GetDoor) "NoCollision")
        (else
          (Collision|SetCollisionEnabled (Variables|Default|GetDoor) "QueryAndPhysics"))))))

(fn ConstructionScript)