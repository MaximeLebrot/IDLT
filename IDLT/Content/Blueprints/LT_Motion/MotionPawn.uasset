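; MotionPawn is a pawn that is moved and turned by tilting its right motion controller.
; Each Tick, MovePlayer turns the controller's relative pitch and roll into forward and right movement input along the mesh's axes, and its yaw into controller yaw input.
; Each axis is scaled linearly and ignored inside a shared SensitivityDeadzone.
; Unconnected debug and earlier movement nodes remain in the event graph.
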(event EventTick
  (params (DeltaSeconds :type Float%20%28single-precision%29))
  ;[1 1 1] Teleportation based
  (CallFunction|MovePlayer))

(event Input|ActionEvents|InputActionResetRotation
  (params (Key :type Key%20Structure :default "None"))
  ;[1 1 1] Teleportation based
)

(fn ConstructionScript)

(fn MovePlayer
  (CallFunction|HandleForwardMovement)
  (CallFunction|HandleRightMovement)
  (CallFunction|HandleTurnMovement))

(fn HandleForwardMovement
  (bind _rightcontroller (Variables|Default|GetRightController))
  (bind _relativerotation (Variables|/Script/Engine.SceneComponent|GetRelativeRotation _rightcontroller))
  (bind _returnvalue (* -1.8e+02 (.pitch _relativerotation)))
  (bind _returnvalue_2 (/ _returnvalue 1e+04))
  (if (> (Math|Float|Absolute(Float) _returnvalue_2) (Variables|Default|GetSensitivityDeadzone))
    (Pawn|Input|AddMovementInput (Math|Vector|GetForwardVector (Variables|Character|GetMesh)) _returnvalue_2 false)))

(fn HandleRightMovement
  (bind _rightcontroller (Variables|Default|GetRightController))
  (bind _relativerotation (Variables|/Script/Engine.SceneComponent|GetRelativeRotation _rightcontroller))
  (bind _returnvalue (* 1.8e+02 (.roll _relativerotation)))
  (bind _returnvalue_2 (/ _returnvalue 1e+04))
  (if (> (Math|Float|Absolute(Float) _returnvalue_2) (Variables|Default|GetSensitivityDeadzone))
    (Pawn|Input|AddMovementInput (Math|Vector|GetRightVector (Variables|Character|GetMesh)) _returnvalue_2 false)))

(fn HandleTurnMovement
  (bind _rightcontroller (Variables|Default|GetRightController))
  (bind _relativerotation (Variables|/Script/Engine.SceneComponent|GetRelativeRotation _rightcontroller))
  (bind _returnvalue (* 1.8e+02 (.yaw _relativerotation)))
  (bind _returnvalue_2 (/ _returnvalue 1e+04))
  (if (> (Math|Float|Absolute(Float) _returnvalue_2) (Variables|Default|GetSensitivityDeadzone))
    (Pawn|Input|AddControllerYawInput _returnvalue_2)))