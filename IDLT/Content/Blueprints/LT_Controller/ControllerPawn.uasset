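; ControllerPawn is a player-controlled pawn that handles walking, strafing, turning and a sprint toggle.
; Forward and right axis inputs add movement along the Mesh's forward and right vectors, scaled by a Speed multiplier.
; Each Sprint press flips the Sprinting flag and switches Speed between half and full input scale.
; The TurnRight axis feeds controller yaw directly, and the file handles no pitch input.
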(event Input|ActionEvents|InputActionSprint
  (params (Key :type Key%20Structure :default "None"))
  ;[1 1 1] Sprint
  (:Pressed
    (if (Variables|Default|GetSprinting)
      (Variables|Default|SetSpeed 0.5)
      (Variables|Default|SetSprinting false)
      (else
        (Variables|Default|SetSpeed 1.0)
        (Variables|Default|SetSprinting true)))))

(event Input|AxisEvents|InputAxisMoveForward
  (params (AxisValue :type Float%20%28single-precision%29))
  ;[1 1 1] Controller-Based
  (Pawn|Input|AddMovementInput (Math|Vector|GetForwardVector (Variables|Character|GetMesh)) (* AxisValue (Variables|Default|GetSpeed)) false))

(event Input|AxisEvents|InputAxisMoveRight
  (params (AxisValue :type Float%20%28single-precision%29))
  ;[1 1 1] Controller-Based
  (Pawn|Input|AddMovementInput (Math|Vector|GetRightVector (Variables|Character|GetMesh)) (* AxisValue (Variables|Default|GetSpeed)) false))

(event Input|AxisEvents|InputAxisTurnRight
  (params (AxisValue :type Float%20%28single-precision%29))
  ;[1 1 1] Controller-Based
  (Pawn|Input|AddControllerYawInput AxisValue))

(fn ConstructionScript)