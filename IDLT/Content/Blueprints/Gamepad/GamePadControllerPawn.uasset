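; A pawn driven by gamepad thumbsticks for movement and looking around.
; The left stick adds movement input along the control rotation's forward and right axes, and the right stick feeds controller yaw and pitch.
; When InvertedControls is set, those movement axes pass through the actor's inverse transform before use, rather than being negated.
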(event Input|GamepadEvents|GamepadRightX
  (params (AxisValue :type Float%20%28single-precision%29))
  ;[1 1 1] Controller-Based
  (Pawn|Input|AddControllerYawInput AxisValue))

(event Input|GamepadEvents|GamepadRightY
  (params (AxisValue :type Float%20%28single-precision%29))
  ;[1 1 1] Controller-Based
  (Pawn|Input|AddControllerPitchInput AxisValue))

(event Input|GamepadEvents|GamepadLeftX
  (params (AxisValue :type Float%20%28single-precision%29))
  ;[1 1 1] Controller-Based
  (if (Variables|Default|GetInvertedControls)
    (Pawn|Input|AddMovementInput (Math|Transform|InverseTransformDirection (Transformation|GetActorTransform) (.Y (Math|Rotator|GetAxes (Pawn|GetControlRotation :!class /Script/Engine.Pawn)))) AxisValue false)
    (else
      (Pawn|Input|AddMovementInput (.Y (Math|Rotator|GetAxes (Pawn|GetControlRotation :!class /Script/Engine.Pawn))) AxisValue false))))

(event Input|GamepadEvents|GamepadLeftY
  (params (AxisValue :type Float%20%28single-precision%29))
  ;[1 1 1] Controller-Based
  (if (Variables|Default|GetInvertedControls)
    (Pawn|Input|AddMovementInput (Math|Transform|InverseTransformDirection (Transformation|GetActorTransform) (.X (Math|Rotator|GetAxes (Pawn|GetControlRotation :!class /Script/Engine.Pawn)))) AxisValue false)
    (else
      (Pawn|Input|AddMovementInput (.X (Math|Rotator|GetAxes (Pawn|GetControlRotation :!class /Script/Engine.Pawn))) AxisValue false))))

(fn ConstructionScript)