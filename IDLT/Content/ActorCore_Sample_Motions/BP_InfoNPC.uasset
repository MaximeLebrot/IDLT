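; Info NPC actor from the ActorCore sample motions folder, built to turn toward a nearby player and toggle a text display.
; Tick calls LookAt while PlayerInRange is true, rotating the actor on yaw only toward PlayerRef.
; InfoRange overlap events are empty and their range-setting nodes are disconnected, so this graph never updates the player state.
; SetTextVisibility, called on BeginPlay, also does nothing because its visibility node is unwired.
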(event OnComponentBeginOverlap(InfoRange)
  (params (OverlappedComponent :type Primitive%20Component%20Object%20Reference) (OtherActor :type Actor%20Object%20Reference) (OtherComp :type Primitive%20Component%20Object%20Reference) (OtherBodyIndex :type Integer) (bFromSweep :type Boolean) (SweepResult :type Hit%20Result%20Structure%20%28by%20ref%29)))

(event OnComponentEndOverlap(InfoRange)
  (params (OverlappedComponent :type Primitive%20Component%20Object%20Reference) (OtherActor :type Actor%20Object%20Reference) (OtherComp :type Primitive%20Component%20Object%20Reference) (OtherBodyIndex :type Integer)))

(event EventBeginPlay
  (CallFunction|SetTextVisibility false))

(event EventTick
  (params (DeltaSeconds :type Float%20%28single-precision%29))
  (if (Variables|Default|GetPlayerInRange)
    (CallFunction|Lookat (Variables|Default|GetPlayerRef))))

(fn ConstructionScript)

(fn SetTextVisibility
  (params (Visible :type Boolean)))

(fn Lookat
  (params (LookAtTarget :type Actor%20Object%20Reference))
  (Transformation|SetActorRotation (Math|Rotator|MakeRotator 0.0 0.0 (.Yaw (Math|Rotator|BreakRotator (Math|Rotator|FindLookatRotation (Transformation|GetActorLocation) (Transformation|GetActorLocation LookAtTarget)))))))