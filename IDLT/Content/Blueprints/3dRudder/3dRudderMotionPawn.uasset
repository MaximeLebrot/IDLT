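; 3dRudder motion pawn that moves and turns the player through axis inputs, based on the 3dRudder controller.
; MoveForward and MoveRight add movement along the actor's forward and right vectors, and TurnRight adds controller yaw, all scaled by a shared Speed variable.
; LookUp is left unwired, so its pitch input node never runs and the pawn has no pitch control.
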(event Input|AxisEvents|InputAxisMoveForward
  (params (AxisValue :type Float%20%28single-precision%29))
  ;[1 1 1] 3dRudder Motion based
  (Pawn|Input|AddMovementInput (Transformation|GetActorForwardVector) (* AxisValue (Variables|Default|GetSpeed)) false))

(event Input|AxisEvents|InputAxisMoveRight
  (params (AxisValue :type Float%20%28single-precision%29))
  ;[1 1 1] 3dRudder Motion based
  (Pawn|Input|AddMovementInput (Transformation|GetActorRightVector) (* AxisValue (Variables|Default|GetSpeed)) false))

(event Input|AxisEvents|InputAxisTurnRight
  (params (AxisValue :type Float%20%28single-precision%29))
  ;[1 1 1] 3dRudder Motion based
  (Pawn|Input|AddControllerYawInput (* AxisValue (Variables|Default|GetSpeed))))

(event Input|AxisEvents|InputAxisLookUp
  (params (AxisValue :type Float%20%28single-precision%29))
  ;[1 1 1] 3dRudder Motion based
)

(fn ConstructionScript)