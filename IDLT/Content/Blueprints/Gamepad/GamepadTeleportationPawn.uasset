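; Gamepad-controlled pawn that moves by arc teleportation, with the right stick turning the view.
; While Teleport is held, Tick predicts a projectile path from the Sphere, with launch direction built from capsule forward plus left-stick input.
; Hits on sufficiently upward-facing surfaces are valid targets, previewed with debug path and sphere drawing.
; On release, the pawn teleports to the last valid hit, raised by capsule half-height.
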(event EventTick
  (params (DeltaSeconds :type Float%20%28single-precision%29))
  (bind _teleportlocation (Variables|Default|GetTeleportLocation))
  ;[1 1 1] Teleportation based
  (Variables|Default|SetDirection (Math|Vector|MakeVector (stale Input|GamepadEvents|GamepadLeftY AxisValue) (stale Input|GamepadEvents|GamepadLeftX AxisValue) 0.0))
  (if (Variables|Default|GetTeleportHold)
    (CallFunction|TraceTeleport)
    (elif (Variables|Default|GetCanTeleport)
      (Transformation|Teleport (Math|Vector|MakeVector (.x _teleportlocation) (.y _teleportlocation) (+ (.z _teleportlocation) (.OutHalfHeight (Components|Capsule|GetScaledCapsuleSize (Variables|Collision|GetCapsuleComponent))))) (Transformation|GetActorRotation))
      (Variables|Default|SetCanTeleport false))))

(event EventBeginPlay
  ;[1 1 1] Teleportation based
  (Variables|Default|SetTeleportLocation (Transformation|GetActorLocation)))

(event Input|ActionEvents|InputActionTeleport
  (params (Key :type Key%20Structure :default "None"))
  ;[1 1 1] Teleportation based
  (:Pressed
    (Variables|Default|SetTeleportHold true))
  (:Released
    (Variables|Default|SetTeleportHold false)))

(event Input|GamepadEvents|GamepadRightX
  (params (AxisValue :type Float%20%28single-precision%29))
  ;[1 1 1] Teleportation based
  (Pawn|Input|AddControllerYawInput AxisValue))

(event Input|GamepadEvents|GamepadRightY
  (params (AxisValue :type Float%20%28single-precision%29))
  ;[1 1 1] Teleportation based
  (Pawn|Input|AddControllerPitchInput AxisValue))

(event Input|GamepadEvents|GamepadLeftX
  (params (AxisValue :type Float%20%28single-precision%29))
  ;[1 1 1] Teleportation based
)

(event Input|GamepadEvents|GamepadLeftY
  (params (AxisValue :type Float%20%28single-precision%29))
  ;[1 1 1] Teleportation based
)

(fn ConstructionScript)

(fn TraceTeleport
  (bind _capsulecomponent (Variables|Collision|GetCapsuleComponent))
  (bind (_outhit _outpathpositions _outlasttracedestination _returnvalue) (Class|GameplayStatics|BlueprintPredictProjectilePathbyObjectType (Transformation|GetWorldLocation (Variables|Default|GetSphere)) (* (+ (Math|Transform|TransformDirection (Transformation|GetWorldTransform _capsulecomponent) (Variables|Default|GetDirection)) (Math|Vector|GetForwardVector (Transformation|GetWorldRotation _capsulecomponent))) (Variables|Default|GetTeleportLength)) true 0.0 (Utilities|Array|MakeArray "ObjectTypeQuery1" "ObjectTypeQuery2") false 0 "ForOneFrame"))
  (if _returnvalue
    (Variables|Default|SetCanTeleport (> (.Z (Math|Vector|BreakVector (.ImpactNormal (Collision|BreakHitResult _outhit)))) 0.5))
    (bind _output_get (Variables|Default|SetTeleportLocation (.ImpactPoint (Collision|BreakHitResult _outhit))))
    (Rendering|Debug|DrawDebugSphere (+ _output_get (Math|Vector|MakeVector 0.0 0.0 15.0)) 15.0 16 "(R=0.130208,G=0.137454,B=1.000000,A=1.000000)" 0.0)))